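; Player pawn with mouse look that moves with the arrow keys and interacts with Item actors in view.
; Arrow keys offset it without sweep along camera axes: Right moves continuously while held, the others step once per press.
; Each tick, a debug-drawn line trace from the camera prints the hit Item's Nome and hides that Item while the left mouse button is held.
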(event `self.ReceiveTick`
  (params (DeltaSeconds :type "Float (single-precision)"))
  (bind _camera (`self.Camera`))
  (bind _returnvalue (`SceneComponent.K2_GetComponentLocation` _camera))
  (if (`self.Right Pressed`)
    (`self.K2_AddActorWorldOffset` (* (`SceneComponent.GetRightVector` (`self.Camera`)) 10)))
  (bind _outhit (`KismetSystemLibrary.LineTraceSingle` :`Start` _returnvalue :`End` (+ _returnvalue (* (`SceneComponent.GetForwardVector` _camera) 1000)) :`TraceChannel` "TraceTypeQuery1" :`DrawDebugType` "ForDuration"))
  (bind _asitem (cast `/Game/Blueprints/Item` (`.HitActor` (`GameplayStatics.BreakHitResult` _outhit))))
  (`KismetSystemLibrary.PrintString` (`/Game/Blueprints/Item.Nome` _asitem))
  (if (`self.Left Mouse Pressed`)
    (`self.SetActorHiddenInGame` _asitem true)))

(event `Key|LeftMouseButton`
  (params (Key :type "Key Structure"))
  (:`Pressed`
    (set `self.Left Mouse Pressed` true))
  (:`Released`
    (set `self.Left Mouse Pressed` false)))

(event `Key|Right`
  (params (Key :type "Key Structure"))
  (:`Pressed`
    (set `self.Right Pressed` true))
  (:`Released`
    (set `self.Right Pressed` false)))

(event `Key|Right`
  (params (Key :type "Key Structure")))

(event `Key|Left`
  (params (Key :type "Key Structure"))
  (:`Pressed`
    (`self.K2_AddActorWorldOffset` (* (`SceneComponent.GetRightVector` (`self.Camera`)) -50))))

(event `Key|Down`
  (params (Key :type "Key Structure"))
  (:`Pressed`
    (`self.K2_AddActorWorldOffset` (* (`SceneComponent.GetForwardVector` (`self.Camera`)) -50))))

(event `Key|Up`
  (params (Key :type "Key Structure"))
  (:`Pressed`
    (`self.K2_AddActorWorldOffset` (* (`SceneComponent.GetForwardVector` (`self.Camera`)) 50))))

(event `InputAxisKey|MouseX`
  (params (AxisValue :type "Float (single-precision)"))
  (`self.AddControllerYawInput` AxisValue))

(event `InputAxisKey|MouseY`
  (params (AxisValue :type "Float (single-precision)"))
  (`self.AddControllerPitchInput` (* -1 AxisValue)))

(fn `UserConstructionScript`)